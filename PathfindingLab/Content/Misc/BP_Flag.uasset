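; BP_Flag is a capture-the-flag pickup that follows its carrier and can be reset to its spawn location.
; When uncaptured, an overlap by a MyCTFActor or CTFAIActor sets that SteeringActor's HasFlag and records it as holder.
; Tick derives IsCaptured from the first two SteeringActors' HasFlag, prints the state, and snaps the flag to the holder while captured.
; ResetFlag clears IsCaptured and restores the initial position, leaving HasFlag untouched.
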(event `self.ReceiveBeginPlay`
  (set `self.IsCaptured` false)
  (set `self.InitialPos` (`self.K2_GetActorLocation`)))

(event `self.CollisionComponent.OnComponentBeginOverlap`
  (params (OverlappedComponent :type "PrimitiveComponent Object Reference") (OtherActor :type "Actor Object Reference") (OtherComp :type "PrimitiveComponent Object Reference") (OtherBodyIndex :type Integer) (bFromSweep :type Boolean) (SweepResult :type "HitResult Structure (by ref)"))
  (bind _returnvalue (`GameplayStatics.GetObjectClass` OtherActor))
  (if (or (== _returnvalue "/Game/SteeringActor/MyCTFActor.MyCTFActor_C") (== _returnvalue "/Game/SteeringActor/CTFAIActor.CTFAIActor_C"))
    (if (not (`self.IsCaptured`))
      (bind _assteering_actor (cast `SteeringActor` OtherActor))
      (set `SteeringActor.hasFlag` true _assteering_actor)
      (set `self.CurrentFlagHolder` OtherActor))))

(event `self.ReceiveTick`
  (params (DeltaSeconds :type "Float (single-precision)"))
  (bind _outactors (`GameplayStatics.GetAllActorsOfClass` "/Script/PathFinding.SteeringActor"))
  (bind _output_get (set `self.IsCaptured` (or (`SteeringActor.hasFlag` (`|GetArrayItem` _outactors)) (`SteeringActor.hasFlag` (`|GetArrayItem` _outactors 1)))))
  (if _output_get
    (`KismetSystemLibrary.PrintString` "Captured" true true (struct :`G` 0.66 :`B` 1.0 :`A` 1.0) 0.0)
    (`self.K2_SetActorLocation` (`self.K2_GetActorLocation` (`self.CurrentFlagHolder`)))
    (else
      (`KismetSystemLibrary.PrintString` "NotCaptured" true true (struct :`G` 0.66 :`B` 1.0 :`A` 1.0) 0.0))))

(event `self.resetFlag`
  (if (`self.IsCaptured`)
    (set `self.IsCaptured` false))
  (`self.K2_SetActorLocation` (`self.InitialPos`)))

(fn `UserConstructionScript`)