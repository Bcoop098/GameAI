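; BP_Player is a player Blueprint whose only active logic is mouse wheel camera zoom.
; Each wheel press steps a clamped Zoom value in or out and writes it directly to the SpringArm's target arm length.
; An unconnected node chain, which never runs, would destroy BP_SteeringActor instances and spawn a new one at a fixed location.
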(event `Key|MouseScrollUp`
  (params (Key :type "Key Structure"))
  (:`Pressed`
    (set `self.Zoom` (`KismetMathLibrary.FClamp` (+ (`self.Zoom`) -100.0) 600.0 3000.0))
    (set `SpringArmComponent.TargetArmLength` (`self.Zoom`) (`self.SpringArm`) :!label _label)))

(event `Key|MouseScrollDown`
  (params (Key :type "Key Structure"))
  (:`Pressed`
    (set `self.Zoom` (`KismetMathLibrary.FClamp` (+ (`self.Zoom`) 100.0) 600.0 3000.0))
    (goto _label)))

(event `Key|F`
  (params (Key :type "Key Structure")))

(fn `UserConstructionScript`)