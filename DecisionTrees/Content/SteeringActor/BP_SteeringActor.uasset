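; Steering agent that follows a grid path to the player's position, computed once shortly after play begins.
; On start it has the MyPathBuilderActor rebuild its grid, respawns Wall actors from the builder's wall list, then requests a path and passes it to path following.
; Each tick it stretches an arrow by steering velocity and draws debug spheres at the target and path points.
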(event `self.ReceiveBeginPlay`
  (bind _pathbuilder (`self.PathBuilder`))
  (bind _walls (`MyPathBuilderActor.Walls` _pathbuilder))
  (`KismetSystemLibrary.Delay` 0.2)
  (bind _outactors (`GameplayStatics.GetAllActorsOfClass` "/Script/PathFinding.MyPathBuilderActor"))
  (set `self.PathBuilder` (`|GetArrayItem` _outactors))
  (`MyPathBuilderActor.changeGrid` _pathbuilder 25)
  (bind _outactors_2 (`GameplayStatics.GetAllActorsOfClass` "/Game/Misc/Wall.Wall_C"))
  (`self.K2_DestroyActor` _outactors_2)
  (for _index (range (+ (`KismetArrayLibrary.Array_Length` _walls) 1))
    (`|SpawnActorFromClass` "/Game/Misc/Wall.Wall_C" (`KismetMathLibrary.Conv_VectorToTransform` (`|GetArrayItem` _walls _index)) "Undefined" "OverrideRootScale" null null))
  (bind _returnvalue (`MyPathBuilderActor.checkPoint` _pathbuilder (/ (`self.K2_GetActorLocation`) 100)))
  (bind _returnvalue_2 (`MyPathBuilderActor.checkPoint` _pathbuilder (/ (`self.K2_GetActorLocation` (`GameplayStatics.GetPlayerPawn` 0)) 100)))
  (bind _returnvalue_3 (`MyPathBuilderActor.getPath` _pathbuilder _returnvalue (`KismetMathLibrary.Conv_VectorToVector2D` _returnvalue_2)))
  (`self.AddToPathFollow` _returnvalue_3))

(event `self.ReceiveTick`
  (params (DeltaSeconds :type "Float (single-precision)"))
  (`self.UpdateArrow`)
  (`self.DisplatPath`))

(fn `DisplatPath`
  (`KismetSystemLibrary.DrawDebugSphere` (`self.TargetPos`) 100.0 12 (struct :`R` 0.117766 :`G` 1.0 :`B` 0.143879 :`A` 1.0))
  (for _array_element (`self.Path`)
    (`KismetSystemLibrary.DrawDebugSphere` _array_element 30.0 12 (struct :`R` 0.356519 :`G` 1.0 :`B` 0.617714 :`A` 1.0))))

(fn `UpdateArrow`
  (`SceneComponent.SetRelativeScale3D` (`self.Arrow`) (`KismetMathLibrary.MakeVector` (`KismetMathLibrary.MapRangeClamped` (`KismetMathLibrary.VSize` (`self.SteeringVelocity`)) 0.0 (`self.MaxSpeed`) 1.0 3.0) 2.0 3.0)))

(fn `UserConstructionScript`)