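; Player pawn that acts as a movable, zoomable camera rig and can reset the steering actors in the level.
; Tick applies left-stick input as a swept world-space XY offset, scaled by Speed and delta time.
; The mouse wheel steps a clamped Zoom value that sets the spring arm length.
; The F key destroys all BP_SteeringActor instances and spawns a fresh one at a fixed location.
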(event `self.ReceiveTick`
  (params (DeltaSeconds :type "Float (single-precision)"))
  (`self.K2_AddActorWorldOffset` (* (* (`KismetMathLibrary.MakeVector` (`self.GetInputAxisValue`) (`self.GetInputAxisValue`)) (`self.Speed`)) DeltaSeconds) true))

(event `Key|MouseScrollUp`
  (params (Key :type "Key Structure"))
  (:`Pressed`
    (set `self.Zoom` (`KismetMathLibrary.FClamp` (+ (`self.Zoom`) -100.0) 600.0 3000.0))
    (set `SpringArmComponent.TargetArmLength` (`self.Zoom`) (`self.SpringArm`) :!label _label)))

(event `Key|MouseScrollDown`
  (params (Key :type "Key Structure"))
  (:`Pressed`
    (set `self.Zoom` (`KismetMathLibrary.FClamp` (+ (`self.Zoom`) 100.0) 600.0 3000.0))
    (goto _label)))

(event `Key|F`
  (params (Key :type "Key Structure"))
  (:`Pressed`
    (bind _outactors (`GameplayStatics.GetAllActorsOfClass` "/Game/SteeringActor/BP_SteeringActor.BP_SteeringActor_C"))
    (`self.K2_DestroyActor` _outactors)
    (`|SpawnActorFromClass` "/Game/SteeringActor/BP_SteeringActor.BP_SteeringActor_C" (`KismetMathLibrary.Conv_VectorToTransform` (`KismetMathLibrary.MakeVector` 200.0 1000.0 70.0)) "Undefined" "OverrideRootScale" null null)))

(fn `UserConstructionScript`)