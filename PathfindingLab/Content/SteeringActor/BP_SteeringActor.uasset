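; Steering agent actor that follows paths from a path builder and draws debug visuals of its movement.
; At BeginPlay, if a random grid point passes CheckPoint, it requests a path from the player pawn's scaled location to another random cell.
; It feeds that same path into path following every second.
; Each tick scales an arrow by steering speed and draws debug spheres at the target and path points.
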(event `self.ReceiveBeginPlay`
  (bind _returnvalue (`KismetMathLibrary.MakeVector2D` (`KismetMathLibrary.Conv_IntToDouble` (`KismetMathLibrary.RandomInteger` 29)) (`KismetMathLibrary.Conv_IntToDouble` (`KismetMathLibrary.RandomInteger` 29))))
  (set `self.BuilderReference` (`self.MypathBuilder`))
  (bind _returnvalue_2 (`MyPathBuilderActor.checkPoint` _returnvalue))
  (if _returnvalue_2
    (bind _returnvalue_3 (`MyPathBuilderActor.getPath` (/ (`self.K2_GetActorLocation` (`GameplayStatics.GetPlayerPawn` 0)) 100) _returnvalue))
    (`self.AddToPathFollow` _returnvalue_3 :!label _label)
    (`KismetSystemLibrary.Delay` 1.0 :!label _label_2)
    (if true
      (goto _label)
      (else
        (goto _label_2)))))

(event `self.ReceiveTick`
  (params (DeltaSeconds :type "Float (single-precision)"))
  (`self.UpdateArrow`)
  (`self.DisplatPath`))

(fn `DisplatPath`
  (`KismetSystemLibrary.DrawDebugSphere` (`self.TargetPos`) 100.0 12 (struct :`R` 0.117766 :`G` 1.0 :`B` 0.143879 :`A` 1.0))
  (for _array_element (`self.Path`)
    (`KismetSystemLibrary.DrawDebugSphere` _array_element 30.0 12 (struct :`R` 0.356519 :`G` 1.0 :`B` 0.617714 :`A` 1.0))))

(fn `UpdateArrow`
  (`SceneComponent.SetRelativeScale3D` (`self.Arrow`) (`KismetMathLibrary.MakeVector` (`KismetMathLibrary.MapRangeClamped` (`KismetMathLibrary.VSize` (`self.SteeringVelocity`)) 0.0 (`self.MaxSpeed`) 1.0 3.0) 2.0 3.0)))

(fn `UserConstructionScript`)