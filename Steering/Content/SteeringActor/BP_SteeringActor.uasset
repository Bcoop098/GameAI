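; Blueprint steering actor that tracks the target position of the player's pawn and the other steering actors in the level.
; On BeginPlay it caches the player-controlled MyPlayerPawn, printing an error if the cast fails, then gathers every SteeringActor after a short delay.
; Each Tick it copies the pawn's target position into TargetPos; no movement logic appears in this graph.
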(event `self.ReceiveBeginPlay`
  (`|ExecutionSequence`
    (:`then_0`
      (bind _asmy_player_pawn (cast `/Game/PlayerController/MyPlayerPawn` (`Controller.K2_GetPawn` (`GameplayStatics.GetPlayerController` 0)))
        (:`then`
          (set `self.PlayerReference` _asmy_player_pawn))
        (:`CastFailed`
          (`KismetSystemLibrary.PrintString` "Error : Could not find valid player pawn in BP_Steeringactor" true true (struct :`R` 1.0 :`G` 0.057028 :`A` 1.0)))))
    (:`then_1`
      (`KismetSystemLibrary.Delay` 0.2)
      (bind _outactors (`GameplayStatics.GetAllActorsOfClass` "/Script/Steering.SteeringActor"))
      (set `self.AllSteeringActors` _outactors))))

(event `self.ReceiveTick`
  (params (DeltaSeconds :type "Float (single-precision)"))
  (bind _playerreference (`self.PlayerReference`))
  (`/Engine/EditorBlueprintResources/StandardMacros.IsValid` _playerreference
    (:`Is Valid`
      (bind _targetpos (`/Game/PlayerController/MyPlayerPawn.GetTargetPosition` _playerreference))
      (set `self.TargetPos` _targetpos))))

(fn `UserConstructionScript`)